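; BP_Bullet_Chien is a weapon projectile that leaves a damage zone where it comes to a stop.
; Its ProjectileMovement component drives the logic: each bounce only prints a debug string, while stopping spawns a BP_DamageZone at the bullet's transform.
; The bullet destroys itself after a short delay following that spawn.
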(event `self.ProjectileMovement.OnProjectileBounce`
  (params (ImpactResult :type "HitResult Structure (by ref)") (ImpactVelocity :type "Vector Structure (by ref)"))
  (`KismetSystemLibrary.PrintString` "boing"))

(event `self.ProjectileMovement.OnProjectileStop`
  (params (ImpactResult :type "HitResult Structure (by ref)"))
  (`|SpawnActorFromClass` "/Game/Game/Blueprints/Weapons/BP_DamageZone.BP_DamageZone_C" (`self.GetTransform`) "Undefined" "MultiplyWithRoot" null null)
  (`KismetSystemLibrary.Delay` 0.2)
  (`self.K2_DestroyActor` self))

(fn `UserConstructionScript`
  (`parent.UserConstructionScript`))