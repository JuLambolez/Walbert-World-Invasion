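; Minigun weapon that auto-fires BP_Bullet projectiles from its Arrow component toward the arrow's facing.
; A looping timer started on BeginPlay calls Fire every Rate seconds if IsAutoFiring is set.
; Fire projects the mouse cursor onto a horizontal plane at muzzle height, timing each bullet's destruction by that distance over its initial speed.
; Right mouse toggles IsAutoFiring, but the running timer never rechecks it.
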(event `Key|RightMouseButton`
  (params (Key :type "Key Structure"))
  ;[1 1 1] structure conditionelle pour arrêt du tir auto (si nécéssaire pour suite jeu)
  (:`Pressed`
    (set `self.IsAutoFiring` false))
  (:`Released`
    (set `self.IsAutoFiring` true)))

(event `self.ReceiveBeginPlay`
  (`parent.ReceiveBeginPlay`)
  (if (`self.IsAutoFiring`)
    ;[1 1 1] tir en rafale de l'arme 1 avec Fire
    (`KismetSystemLibrary.K2_SetTimer` null "Fire" (`self.Rate`) true)))

(event `self.ReceiveTick`
  (params (DeltaSeconds :type "Float (single-precision)"))
  (`parent.ReceiveTick` DeltaSeconds))

(fn `Fire`
  (bind _returnvalue (`GameplayStatics.GetPlayerController` 0))
  (bind _arrow (`self.Arrow`))
  (bind _returnvalue_2 (`SceneComponent.K2_GetComponentLocation` _arrow))
  (bind (_locationx _locationy) (`PlayerController.GetMousePosition` _returnvalue))
  (bind (_worldposition _worlddirection) (`GameplayStatics.DeprojectScreenToWorld` _returnvalue (`KismetMathLibrary.MakeVector2D` _locationx _locationy)))
  ;[1 1 1] Comment
  (bind _returnvalue_3 (`|SpawnActorFromClass` "/Game/Game/Blueprints/Weapons/BP_Bullet.BP_Bullet_C" (`KismetMathLibrary.MakeTransform` _returnvalue_2 (`SceneComponent.K2_GetComponentRotation` _arrow)) "Undefined" "MultiplyWithRoot" null null))
  (`/Game/Game/Blueprints/Weapons/BP_Bullet.DelayedDestroy` _returnvalue_3 (/ (`KismetMathLibrary.Vector_Distance` _returnvalue_2 (`.Intersection` (`KismetMathLibrary.LinePlaneIntersection` _worldposition (+ _worldposition (* _worlddirection 10000.0)) (`KismetMathLibrary.MakePlaneFromPointAndNormal` _returnvalue_2 (0.0 0.0 1.0))))) (`ProjectileMovementComponent.InitialSpeed` (`/Game/Game/Blueprints/Weapons/BP_Bullet.ProjectileMovement` _returnvalue_3)))))

(fn `UserConstructionScript`
  (`parent.UserConstructionScript`))