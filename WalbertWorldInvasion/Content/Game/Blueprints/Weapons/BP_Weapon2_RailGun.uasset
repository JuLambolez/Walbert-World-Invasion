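; Railgun weapon Blueprint that fires by spawning a BP_BigLaser actor at the location and rotation of its ArrowRailGun component.
; The SpawnLaser event and GoLaser function duplicate this spawn logic, with no caller for either in this file.
; An author note marks the intended E-key trigger as not working, and an endpoint calculation from RangeRailGun is left unused.
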(event `SpawnLaser`
  (bind _arrowrailgun (`self.ArrowRailGun`))
  ;[1 1 1] un laser spawn quand on appuie sur E (MARCHE PAS)
  (`|SpawnActorFromClass` "/Game/Game/Blueprints/Weapons/BP_BigLaser.BP_BigLaser_C" (`KismetMathLibrary.MakeTransform` (`SceneComponent.K2_GetComponentLocation` _arrowrailgun) (`SceneComponent.K2_GetComponentRotation` _arrowrailgun)) "Undefined" "MultiplyWithRoot" null null))

(event `self.ReceiveBeginPlay`
  (`parent.ReceiveBeginPlay`))

(fn `GoLaser`
  (bind _arrowrailgun (`self.ArrowRailGun`))
  (`|SpawnActorFromClass` "/Game/Game/Blueprints/Weapons/BP_BigLaser.BP_BigLaser_C" (`KismetMathLibrary.MakeTransform` (`SceneComponent.K2_GetComponentLocation` _arrowrailgun) (`SceneComponent.K2_GetComponentRotation` _arrowrailgun)) "Undefined" "MultiplyWithRoot" null null))

(fn `UserConstructionScript`
  (`parent.UserConstructionScript`))