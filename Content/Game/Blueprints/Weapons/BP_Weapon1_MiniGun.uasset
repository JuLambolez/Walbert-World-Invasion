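; BP_Weapon1_MiniGun is a minigun weapon that automatically fires bullets at a fixed rate.
; BeginPlay starts a looping timer on Fire when IsAutoFiring is set.
; Fire spawns a BP_Bullet at the Arrow component and calls MoveTo toward a point Range units forward.
; Right mouse press and release toggle IsAutoFiring, but the flag is only read at BeginPlay, so the running timer is unaffected.
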(event `Key|RightMouseButton`
  (params (Key :type "Key Structure"))
  ;[1 1 1] structure conditionelle pour arrêt du tir auto (si nécéssaire pour suite jeu)
  (:`Pressed`
    (set `self.IsAutoFiring` false))
  (:`Released`
    (set `self.IsAutoFiring` true)))

(event `self.ReceiveBeginPlay`
  (`parent.ReceiveBeginPlay`)
  (if (`self.IsAutoFiring`)
    ;[1 1 1] tir en rafale de l'arme 1 avec Fire
    (`KismetSystemLibrary.K2_SetTimer` null "Fire" (`self.Rate`) true)))

(fn `Fire`
  (bind _arrow (`self.Arrow`))
  (bind _arrow_2 (`self.Arrow`))
  (bind _returnvalue (`|SpawnActorFromClass` "/Game/Game/Blueprints/Weapons/BP_Bullet.BP_Bullet_C" (`KismetMathLibrary.MakeTransform` (`SceneComponent.K2_GetComponentLocation` _arrow_2) (`SceneComponent.K2_GetComponentRotation` _arrow_2)) "Undefined" "MultiplyWithRoot" null null))
  (`/Game/Game/Blueprints/Weapons/BP_Bullet.MoveTo` _returnvalue (+ (`SceneComponent.K2_GetComponentLocation` _arrow) (* (`SceneComponent.GetForwardVector` _arrow) (`self.Range`))) 1.0))

(fn `UserConstructionScript`
  (`parent.UserConstructionScript`))