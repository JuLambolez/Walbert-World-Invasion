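; Railgun weapon Blueprint that fires by spawning a BP_BigLaser actor at its ArrowRailGun component's world location and rotation.
; The GoLaser function performs the spawn, and an E key event repeats the same logic directly, noted in French as not working.
; An end-point calculation from the arrow's forward vector and RangeRailGun is left unused.
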(event `Key|E`
  (params (Key :type "Key Structure"))
  (bind _arrowrailgun (`self.ArrowRailGun`))
  ;[1 1 1] un laser spawn quand on appuie sur E (MARCHE PAS)
  (:`Pressed`
    (`|SpawnActorFromClass` "/Game/Game/Blueprints/Weapons/BP_BigLaser.BP_BigLaser_C" (`KismetMathLibrary.MakeTransform` (`SceneComponent.K2_GetComponentLocation` _arrowrailgun) (`SceneComponent.K2_GetComponentRotation` _arrowrailgun)) "Undefined" "MultiplyWithRoot" null null)))

(event `self.ReceiveBeginPlay`
  (`parent.ReceiveBeginPlay`))

(fn `GoLaser`
  (bind _arrowrailgun (`self.ArrowRailGun`))
  (`|SpawnActorFromClass` "/Game/Game/Blueprints/Weapons/BP_BigLaser.BP_BigLaser_C" (`KismetMathLibrary.MakeTransform` (`SceneComponent.K2_GetComponentLocation` _arrowrailgun) (`SceneComponent.K2_GetComponentRotation` _arrowrailgun)) "Undefined" "MultiplyWithRoot" null null))

(fn `UserConstructionScript`
  (`parent.UserConstructionScript`))